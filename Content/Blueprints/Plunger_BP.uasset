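; Pinball-style plunger actor that animates its pull and release and supplies a ball spawn point.
; PlungerCharge plays a timeline that lerps the mesh along its local Y axis from the rest position.
; PlungerStop halts the timeline and quickly snaps the mesh back with MoveComponentTo.
; GetBallWorldLocaiton converts the local BallSpawnLocation to world space through the actor transform.
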(event `PlungerCharge`
  (bind (_direction _changealpha) (`Timeline|Charge Timeline` :!via `PlayFromStart` :!label _label)
    (:`Update`
      (`SceneComponent.K2_SetRelativeLocation` (`self.PlungerMesh`) (`KismetMathLibrary.VLerp` (0.0 0.0 0.0) (0.0 500.0 0.0) _changealpha) false false))))

(event `PlungerStop`
  (`|ExecutionSequence`
    (:`then_0`
      (goto _label :!via `Stop`))
    (:`then_1`
      (`KismetSystemLibrary.MoveComponentTo` (`self.PlungerMesh`) (0.0 0.0 0.0) (struct) false false 0.05))))

(fn `GetBallWorldLocaiton`
  (returns (`Ball Spawn Location` :type "Vector Structure"))
  (return (`KismetMathLibrary.TransformLocation` (`self.GetTransform`) (`self.BallSpawnLocation`))))

(fn `UserConstructionScript`)