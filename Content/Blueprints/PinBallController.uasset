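; Player controller for a pinball game that turns player input into flipper and plunger actions.
; On BeginPlay it finds all flipper actors, sorting them into left and right arrays by FlipType, and caches the first plunger found.
; Input press and release drive Flip and Flop on each side's flippers and charge or stop the plunger.
; A CreateHUD event clears existing widgets and adds a new pinball HUD to the viewport.
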(event `Create HUD`
  (`WidgetLayoutLibrary.RemoveAllWidgets`)
  (bind _returnvalue (`|CreateWidget` "/Game/Blueprints/UI/PinBallHUD.PinBallHUD_C"))
  (`UserWidget.AddToViewport` _returnvalue 0))

(event `self.ReceiveBeginPlay`
  (`self.GetFlippers`)
  (`self.GetPlunger`))

(event `InputAction|RightFlipper_Input`
  (params (Key :type "Key Structure"))
  (:`Pressed`
    (for _array_element (`self.RightFlippers`)
      (`/Game/Blueprints/Flipper_BP.Flip` _array_element)))
  (:`Released`
    (for _array_element_2 (`self.RightFlippers`)
      (`/Game/Blueprints/Flipper_BP.Flop` _array_element_2))))

(event `InputAction|LeftFlipper_Input`
  (params (Key :type "Key Structure"))
  (:`Pressed`
    (for _array_element (`self.LeftFlippers`)
      (`/Game/Blueprints/Flipper_BP.Flip` _array_element)))
  (:`Released`
    (for _array_element_2 (`self.LeftFlippers`)
      (`/Game/Blueprints/Flipper_BP.Flop` _array_element_2))))

(event `InputAction|PlungerCharge_Input`
  (params (Key :type "Key Structure"))
  (bind _plunger (`self.Plunger`))
  (:`Pressed`
    (`/Game/Blueprints/Plunger_BP.PlungerCharge` _plunger))
  (:`Released`
    (`/Game/Blueprints/Plunger_BP.PlungerStop` _plunger)))

(event `GetFlippers`
  (bind _outactors (`GameplayStatics.GetAllActorsOfClass` "/Game/Blueprints/Flipper_BP.Flipper_BP_C"))
  (for _array_element _outactors
    (switch `/Game/Blueprints/FlipDirection` (`/Game/Blueprints/Flipper_BP.FlipType` _array_element)
      (:`NewEnumerator0`
        (`KismetArrayLibrary.Array_Add` (`self.LeftFlippers`) _array_element))
      (:`NewEnumerator1`
        (`KismetArrayLibrary.Array_Add` (`self.RightFlippers`) _array_element)))))

(event `GetPlunger`
  (bind _outactors (`GameplayStatics.GetAllActorsOfClass` "/Game/Blueprints/Plunger_BP.Plunger_BP_C"))
  (set `self.Plunger` (`|GetArrayItem` _outactors)))

(fn `UserConstructionScript`)