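; Rail actor that builds a mesh track along an editable spline in its Construction Script, with no active runtime logic.
; It adds one spline mesh component per segment, fitting each to the local location and tangent of its two bounding spline points.
; The first segment uses the start mesh with a configurable start scale, the last uses the end mesh, and those between use the mid mesh.
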(fn `UserConstructionScript`
  (locals (SplineMeshVar :type "SplineMeshComponent Object Reference"))
  (bind _spline (`self.Spline`))
  (bind _startscale (`self.StartScale`))
  (bind _returnvalue (- (`SplineComponent.GetNumberOfSplinePoints` (`self.Spline`)) 2))
  (for _index (range (+ _returnvalue 1))
    (bind _returnvalue_2 (`AddComponent|NODE_AddSplineMeshComponent-0`))
    (set `local.SplineMeshVar` _returnvalue_2)
    (if (== _index 0)
      (`StaticMeshComponent.SetStaticMesh` (`local.SplineMeshVar`) (`self.StartMesh`))
      (`SplineMeshComponent.SetStartScale` (`local.SplineMeshVar`) (`KismetMathLibrary.MakeVector2D` _startscale _startscale) true)
      (elif (== _index _returnvalue)
        (`StaticMeshComponent.SetStaticMesh` (`local.SplineMeshVar`) (`self.EndMesh`))
        (else
          (`StaticMeshComponent.SetStaticMesh` (`local.SplineMeshVar`) (`self.MidMesh`)))))
    (bind (_location _tangent) (`SplineComponent.GetLocationAndTangentAtSplinePoint` _spline _index "Local"))
    (bind (_location_2 _tangent_2) (`SplineComponent.GetLocationAndTangentAtSplinePoint` _spline (+ _index 1) "Local"))
    (`SplineMeshComponent.SetStartAndEnd` (`local.SplineMeshVar`) _location _tangent _location_2 _tangent_2 true)))