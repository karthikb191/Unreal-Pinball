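; Pinball slingshot bumper that kicks an overlapping Ball_BP away and adds score through GameMode_PB.
; On overlap it plays an attached sound and applies a mass-independent horizontal impulse along the capsule's negative forward vector.
; A timeline drives the band's deformation through a scalar morph parameter on a dynamic material instance created in the construction script.
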(event `self.ReceiveActorBeginOverlap`
  (params (OtherActor :type "Actor Object Reference"))
  (bind (_returnvalue_x _returnvalue_y) (`KismetMathLibrary.BreakVector` (* (`SceneComponent.GetForwardVector` (`self.Capsule`)) -5000.0)))
  (bind _asball_bp (cast `/Game/Blueprints/Ball_BP` OtherActor))
  (bind _ball (`/Game/Blueprints/Ball_BP.Ball` _asball_bp))
  (`GameplayStatics.SpawnSoundAttached` "/Game/Assets/Sounds/SlingShotCue.SlingShotCue" _ball "None" (0.0 0.0 0.0) (struct) "KeepRelativeOffset" false 1.0 1.0 0.0 null null)
  (bind _asgame_mode_pb (cast `/Game/Blueprints/GameMode_PB` (`GameplayStatics.GetGameMode`))
    (:`then`
      (`/Game/Blueprints/GameMode_PB.AddScore` _asgame_mode_pb 50))
    (:`CastFailed`
      _))
  (`PrimitiveComponent.AddImpulse` _ball (`KismetMathLibrary.MakeVector` _returnvalue_x _returnvalue_y) "None" true)
  (bind (_direction _slipanimalpha) (`Timeline|SlingAnim` :!via `PlayFromStart`)
    (:`Update`
      (bind _asmaterial_instance_dynamic (cast `MaterialInstanceDynamic` (`PrimitiveComponent.GetMaterial` (`self.SlingShotMesh`) 2)))
      (`MaterialInstanceDynamic.SetScalarParameterValue` _asmaterial_instance_dynamic "BandMorphOffset" _slipanimalpha))))

(fn `UserConstructionScript`
  (`PrimitiveComponent.CreateDynamicMaterialInstance` (`self.SlingShotMesh`) 2 null "None"))