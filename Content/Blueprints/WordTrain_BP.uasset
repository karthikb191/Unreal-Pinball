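; WordTrain actor that builds a straight span of meshes between StartMesh and an EndPoint, with no active gameplay logic.
; The construction script turns StartMesh toward EndPoint and adds an EndMesh there, facing back.
; It adds a middle mesh at the start, aimed at the end and stretched along X by the distance over 100, implying a 100-unit-long source mesh.
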(fn `UserConstructionScript`
  (bind _startmesh (`self.StartMesh`))
  (bind _endpoint (`self.EndPoint`))
  (bind _startmesh_2 (`self.StartMesh`))
  (bind _relativelocation (`SceneComponent.RelativeLocation` _startmesh))
  (bind _relativelocation_2 (`SceneComponent.RelativeLocation` (`self.StartMesh`)))
  (`SceneComponent.K2_SetRelativeRotation` _startmesh_2 (`KismetMathLibrary.FindLookAtRotation` (`SceneComponent.RelativeLocation` _startmesh_2) (`self.EndPoint`)) false false)
  (bind _returnvalue (`AddComponent|NODE_AddStaticMeshComponent-2` :`RelativeTransform` (`SceneComponent.GetRelativeTransform` _startmesh)))
  (bind _output_get (set `self.EndMesh` _returnvalue))
  (`SceneComponent.K2_SetRelativeLocationAndRotation` _output_get _endpoint (`KismetMathLibrary.FindLookAtRotation` _endpoint _relativelocation) false false)
  (bind _returnvalue_2 (`AddComponent|NODE_AddStaticMeshComponent-3`))
  (`SceneComponent.K2_SetRelativeTransform` _returnvalue_2 (`KismetMathLibrary.MakeTransform` _relativelocation_2 (`KismetMathLibrary.FindLookAtRotation` _relativelocation_2 (`self.EndPoint`)) (`KismetMathLibrary.MakeVector` (/ (`KismetMathLibrary.VSize` (- _endpoint _relativelocation)) 100.0) 1.0 1.0)) false false))