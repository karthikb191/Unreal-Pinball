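; Pinball game mode that runs the session: main menu and music on start, ball spawning, scoring and game over.
; Balls spawn at the first plunger, and each destroyed ball uses up a try or ends the game.
; Game over opens high score entry if the cached HighScoreSave has room or a lower score, else the main menu.
; Reset restores class defaults, spawns a ball, rebuilds the HUD and broadcasts OnGameReset.
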(event `self.ReceiveBeginPlay`
  (`self.CreateMainMenu`)
  (`GameplayStatics.PlaySound2D` "/Game/Assets/Sounds/victoryMusic_loop_01_01.victoryMusic_loop_01_01" 1.0 1.0 0.0 null null))

(event `SpawnBall`
  (bind _outactors (`GameplayStatics.GetAllActorsOfClass` "/Game/Blueprints/Plunger_BP.Plunger_BP_C"))
  (bind _returnvalue (`|SpawnActorFromClass` "/Game/Blueprints/Ball_BP.Ball_BP_C" (`KismetMathLibrary.MakeTransform` (`/Game/Blueprints/Plunger_BP.GetBallWorldLocaiton` (`|GetArrayItem` _outactors))) "Undefined" "OverrideRootScale" null null))
  (add `self.OnDestroyed` _returnvalue (delegate `OnBalDestroyed`)))

(event `OnBalDestroyed` :!signature `self.OnDestroyed`
  (params (DestroyedActor :type "Actor Object Reference"))
  (if (> (`self.TriesLeft`) 0)
    (`/Engine/EditorBlueprintResources/StandardMacros.DecrementInt` (`self.TriesLeft`)
      (:`  `
        (`self.SpawnBall`)))
    (else
      (`self.EndGame`))))

(event `EndGame`
  (bind _currentsaveobject (`self.GetSaveGameData`))
  (if (<= (`KismetArrayLibrary.Array_Length` (`/Game/Blueprints/HighScoreSave.SaveStruct` _currentsaveobject)) 3)
    (`self.CreateHighScoreWidget` :!label _label)
    (else
      (bind _lowestscorestruct (`/Game/Blueprints/HighScoreSave.DetermineLowestScore` _currentsaveobject))
      (if (< (`.Score_5_643368FF473A0BB313CD35B5164D1580` (break `/Game/Blueprints/HighScoreStruct` _lowestscorestruct)) (`self.Score`))
        (goto _label)
        (else
          (`self.CreateMainMenu`))))))

(event `ResetGame`
  (bind (_score _multiplier _triesleft) (defaults `/Game/Blueprints/GameMode_PB` "GameMode_PB_C"))
  (bind _aspin_ball_controller (cast `/Game/Blueprints/PinBallController` (`GameplayStatics.GetPlayerController` 0) :!pure true))
  (set `self.Score` _score)
  (set `self.Multiplier` _multiplier)
  (set `self.TriesLeft` _triesleft)
  (`self.SpawnBall`)
  (`/Game/Blueprints/PinBallController.Create HUD` _aspin_ball_controller)
  (set `PlayerController.bShowMouseCursor` false _aspin_ball_controller)
  (`self.OnGameReset`))

(event `CreateHighScoreWidget`
  (bind _aspin_ball_controller (cast `/Game/Blueprints/PinBallController` (`GameplayStatics.GetPlayerController` 0)))
  (bind _returnvalue (`|CreateWidget` "/Game/Blueprints/UI/HighScoreEntry.HighScoreEntry_C" _aspin_ball_controller))
  (`UserWidget.AddToViewport` _returnvalue 0)
  (set `PlayerController.bShowMouseCursor` true _aspin_ball_controller))

(event `CreateMainMenu`
  (bind _aspin_ball_controller (cast `/Game/Blueprints/PinBallController` (`GameplayStatics.GetPlayerController` 0)))
  (bind _returnvalue (`|CreateWidget` "/Game/Blueprints/UI/MainMenu.MainMenu_C" _aspin_ball_controller))
  (`UserWidget.AddToViewport` _returnvalue 0)
  (set `PlayerController.bShowMouseCursor` true _aspin_ball_controller))

(fn `AddScore`
  (params (ScoreToAdd :type Integer))
  (returns (NewScore :type Integer))
  (bind _output_get (set `self.Score` (+ (* ScoreToAdd (`self.Multiplier`)) (`self.Score`))))
  (return _output_get))

(fn `GetSaveGameData`
  (returns (currentSaveObject :type "/Game/Blueprints/HighScoreSave Object Reference"))
  (bind _currentsavedata (`self.CurrentSaveData`)
    (:`then`
      (return _currentsavedata))
    (:`else`
      (bind _returnvalue (`GameplayStatics.DoesSaveGameExist` (`self.HighScoreSaveName`)))
      (if _returnvalue
        (bind _returnvalue_2 (`GameplayStatics.LoadGameFromSlot` (`self.HighScoreSaveName`)))
        (bind _ashigh_score_save (cast `/Game/Blueprints/HighScoreSave` _returnvalue_2)
          (:`then`
            (`/Game/Blueprints/HighScoreSave.SortScores` _ashigh_score_save)
            (bind _output_get (set `self.CurrentSaveData` _ashigh_score_save))
            (return _output_get))
          (:`CastFailed`
            _))
        (else
          (bind _returnvalue_3 (`GameplayStatics.CreateSaveGameObject` "/Game/Blueprints/HighScoreSave.HighScoreSave_C"))
          (bind _ashigh_score_save_2 (cast `/Game/Blueprints/HighScoreSave` _returnvalue_3)
            (:`then`
              (bind _output_get_2 (set `self.CurrentSaveData` _ashigh_score_save_2))
              (return _output_get_2))
            (:`CastFailed`
              _))))
      (return null))))

(fn `UserConstructionScript`)