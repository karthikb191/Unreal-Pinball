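; Pinball flipper actor that serves as either a left or right flipper, chosen by FlipType.
; The construction script sets mirrored start and end rotations from FlipType, applies the start rotation, and flips the mesh's X scale for the right side.
; Flip plays an attached sound, currently the left flipper cue for both sides, and rotates the flipper to its end rotation over FlipTime.
; Flop rotates it back to the start rotation.
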(event `Flip`
  (bind _flipper (`self.Flipper`))
  (switch `/Game/Blueprints/FlipDirection` (`self.FlipType`)
    (:`NewEnumerator0`
      (`GameplayStatics.SpawnSoundAttached` "/Game/Assets/Sounds/Pinball_FlipperLeft_Cue.Pinball_FlipperLeft_Cue" _flipper "None" (0.0 0.0 0.0) (struct) "KeepRelativeOffset" false 1.0 1.0 0.0 null null))
    (:`NewEnumerator1`
      (`GameplayStatics.SpawnSoundAttached` "/Game/Assets/Sounds/Pinball_FlipperLeft_Cue.Pinball_FlipperLeft_Cue" _flipper "None" (0.0 0.0 0.0) (struct) "KeepRelativeOffset" false 1.0 1.0 0.0 null null)))
  (`KismetSystemLibrary.MoveComponentTo` _flipper (0.0 0.0 0.0) (`self.EndRotation`) false false (`self.FlipTime`)))

(event `Flop`
  (`KismetSystemLibrary.MoveComponentTo` (`self.Flipper`) (0.0 0.0 0.0) (`self.StartRotation`) false false (`self.FlipTime`)))

(fn `UserConstructionScript`
  (set `self.StartRotation` (select `/Game/Blueprints/FlipDirection` (`self.FlipType`) :`NewEnumerator0` (struct :`Yaw` 20.0) :`NewEnumerator1` (struct :`Yaw` -20.0) :!type "Rotator Structure"))
  (set `self.EndRotation` (select `/Game/Blueprints/FlipDirection` (`self.FlipType`) :`NewEnumerator0` (struct :`Yaw` -20.0) :`NewEnumerator1` (struct :`Yaw` 20.0) :!type "Rotator Structure"))
  (`SceneComponent.K2_SetRelativeRotation` (`self.Flipper`) (`self.StartRotation`) false false)
  (switch `/Game/Blueprints/FlipDirection` (`self.FlipType`)
    (:`NewEnumerator0`
      (`SceneComponent.SetRelativeScale3D` (`self.Flipper`) (1.0 1.0 1.0)))
    (:`NewEnumerator1`
      (`SceneComponent.SetRelativeScale3D` (`self.Flipper`) (-1.0 1.0 1.0)))))