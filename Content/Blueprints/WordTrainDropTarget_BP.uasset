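; Pinball word drop-target bank that raises the game mode's Multiplier once every letter of its word is knocked down.
; The construction script spawns a DropTarget_BP child actor per uppercased DropString character, spacing them by the StartMesh-to-EndMesh distance and binding each drop event.
; ProcessDropTargets decrements TargetCounter and increments Multiplier at zero.
; Reset, bound to the game mode's OnGameReset, refills the counter from the word length.
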(event `self.ReceiveBeginPlay`
  (`parent.ReceiveBeginPlay`)
  (bind _asgame_mode_pb (cast `/Game/Blueprints/GameMode_PB` (`GameplayStatics.GetGameMode`)))
  (add `/Game/Blueprints/GameMode_PB.OnGameReset` _asgame_mode_pb (delegate `Reset`)))

(event `Reset`
  (set `self.TargetCounter` (`KismetStringLibrary.Len` (`self.DropString`))))

(event `ProcessDropTargets`
  (bind _result (`/Engine/EditorBlueprintResources/StandardMacros.DecrementInt` (`self.TargetCounter`))
    (:`  `
      (if (== _result 0)
        (bind _asgame_mode_pb (cast `/Game/Blueprints/GameMode_PB` (`GameplayStatics.GetGameMode`)))
        (`/Engine/EditorBlueprintResources/StandardMacros.IncrementInt` (`/Game/Blueprints/GameMode_PB.Multiplier` _asgame_mode_pb))))))

(fn `UserConstructionScript`
  (bind _startmesh (`self.StartMesh`))
  (bind _relativerotation (`SceneComponent.RelativeRotation` _startmesh))
  (`parent.UserConstructionScript`)
  (bind _output_get (set `self.DropString` (`KismetStringLibrary.ToUpper` (`self.DropString`))))
  (bind _returnvalue (`KismetStringLibrary.GetCharacterArrayFromString` _output_get))
  (for (_array_element _array_index) _returnvalue
    (bind _returnvalue_2 (`AddComponent|NODE_AddChildActorComponent-0` :`RelativeTransform` (`KismetMathLibrary.MakeTransform` (+ (* (`KismetMathLibrary.Conv_RotatorToVector` _relativerotation) (* (+ _array_index 1) (/ (`KismetMathLibrary.VSize` (- (`SceneComponent.RelativeLocation` (`self.StartMesh`)) (`SceneComponent.RelativeLocation` (`self.EndMesh`)))) (`KismetMathLibrary.Conv_IntToDouble` (+ (`KismetArrayLibrary.Array_Length` _returnvalue) 1))))) (* (`SceneComponent.GetRightVector` _startmesh) 20.0)) _relativerotation)))
    (bind _asdrop_target_bp (cast `/Game/Blueprints/DropTarget_BP` (`ChildActorComponent.ChildActor` _returnvalue_2)))
    (bind _output_get_2 (set `/Game/Blueprints/DropTarget_BP.DropLetter` _array_element _asdrop_target_bp))
    (`TextRenderComponent.K2_SetText` (`/Game/Blueprints/DropTarget_BP.TextRender` _asdrop_target_bp) (`KismetTextLibrary.Conv_StringToText` _output_get_2))
    (add `/Game/Blueprints/DropTarget_BP.OnDropTarget` _asdrop_target_bp (`|CreateDelegate` :!event `ProcessDropTargets`))))