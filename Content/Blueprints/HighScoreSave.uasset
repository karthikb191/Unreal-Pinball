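; High-score save Blueprint that holds a list of score structs, trimmed to at most four after each addition.
; AddHighScore appends an entry and calls SortScores, a selection-style sort intended to order scores highest first through a temporary array.
; DetermineHighestScore always returns index 0, so the sort removes the wrong element, and the temporary array is never cleared.
; DetermineLowestScore finds the minimum but is not called here.
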(fn `AddHighScore`
  (params (NewScore :type "/Game/Blueprints/HighScoreStruct Structure"))
  (bind _savestruct (`self.SaveStruct`))
  (`KismetArrayLibrary.Array_Add` (`self.SaveStruct`) NewScore)
  (`KismetSystemLibrary.PrintString` null)
  (`self.SortScores`)
  (`KismetArrayLibrary.Array_Resize` _savestruct (`KismetMathLibrary.Min` 4 (`KismetArrayLibrary.Array_Length` _savestruct))))

(fn `DetermineHighestScore`
  (returns (HighestScoreStruct :type "/Game/Blueprints/HighScoreStruct Structure") (HighestScoreIndex :type Integer))
  (locals (HighestScore :type Integer) (HighestIndex :type Integer))
  (for (_array_element _array_index) (`self.SaveStruct`)
    (if (== _array_index 0)
      (set `local.HighestIndex` _array_index)
      (set `local.HighestScore` (`.Score_5_643368FF473A0BB313CD35B5164D1580` (break `/Game/Blueprints/HighScoreStruct` _array_element)))
      (elif (> (`.Score_5_643368FF473A0BB313CD35B5164D1580` (break `/Game/Blueprints/HighScoreStruct` _array_element)) (`local.HighestScore`))
        (set `local.HighestScore` (`.Score_5_643368FF473A0BB313CD35B5164D1580` (break `/Game/Blueprints/HighScoreStruct` _array_element)))
        (set `local.HighestIndex` _array_index))))
  (return (`|GetArrayItem` (`self.SaveStruct`) (`local.HighestIndex`)) 0))

(fn `DetermineLowestScore`
  (returns (LowestScoreStruct :type "/Game/Blueprints/HighScoreStruct Structure") (LowestScoreIndex :type Integer))
  (locals (LowestScore :type Integer) (LowestIndex :type Integer))
  (bind _lowestindex (`local.LowestIndex`))
  (for (_array_element _array_index) (`self.SaveStruct`)
    (if (== _array_index 0)
      (set `local.LowestIndex` _array_index)
      (set `local.LowestScore` (`.Score_5_643368FF473A0BB313CD35B5164D1580` (break `/Game/Blueprints/HighScoreStruct` _array_element)))
      (elif (< (`.Score_5_643368FF473A0BB313CD35B5164D1580` (break `/Game/Blueprints/HighScoreStruct` _array_element)) (`local.LowestScore`))
        (set `local.LowestScore` (`.Score_5_643368FF473A0BB313CD35B5164D1580` (break `/Game/Blueprints/HighScoreStruct` _array_element)))
        (set `local.LowestIndex` _array_index))))
  (return (`|GetArrayItem` (`self.SaveStruct`) _lowestindex) _lowestindex))

(fn `SortScores`
  (locals (tempSaveStruct :type "Array of /Game/Blueprints/HighScoreStruct Structure"))
  (while (> (`KismetArrayLibrary.Array_Length` (`self.SaveStruct`)) 0)
    (bind (_highestscorestruct _highestscoreindex) (`self.DetermineHighestScore`))
    (`KismetArrayLibrary.Array_Add` (`local.tempSaveStruct`) _highestscorestruct)
    (`KismetArrayLibrary.Array_Remove` (`self.SaveStruct`) _highestscoreindex))
  (set `self.SaveStruct` (`local.tempSaveStruct`)))