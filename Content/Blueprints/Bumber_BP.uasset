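; Pinball bumper actor that knocks an overlapping Ball_BP away and awards score through GameMode_PB.
; The overlap calls Bump, which applies a horizontal velocity-change impulse away from the bumper center and plays a hit sound.
; A BumpAmount timeline then drives the mechanism's vertical movement, a point light flash and an emissive boost on the top sticker.
; The construction script creates the dynamic material instance used for that glow.
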(event `self.ReceiveActorBeginOverlap`
  (params (OtherActor :type "Actor Object Reference"))
  (bind _asball_bp (cast `/Game/Blueprints/Ball_BP` OtherActor)) ; Checks if the other actor is a ball
  (`self.Bump` _asball_bp))

(event `Bump`
  (params (Ball :type "/Game/Blueprints/Ball_BP Object Reference"))
  (bind (_returnvalue_x _returnvalue_y) (`KismetMathLibrary.BreakVector` (* (`KismetMathLibrary.GetDirectionUnitVector` (`self.K2_GetActorLocation`) (`self.K2_GetActorLocation` Ball)) 5000.0)))
  (`PrimitiveComponent.AddImpulse` (`/Game/Blueprints/Ball_BP.Ball` Ball) (`KismetMathLibrary.MakeVector` _returnvalue_x _returnvalue_y) "None" true)
  (`GameplayStatics.SpawnSoundAttached` "/Game/Assets/Sounds/BumperHit_Cue.BumperHit_Cue" (`self.BumperHead`) "None" (0.0 0.0 0.0) (struct) "KeepRelativeOffset" false 1.0 1.0 0.0 null null)
  (bind _asgame_mode_pb (cast `/Game/Blueprints/GameMode_PB` (`GameplayStatics.GetGameMode`))
    (:`then`
      (`/Game/Blueprints/GameMode_PB.AddScore` _asgame_mode_pb 10)
      (bind (_direction _bumpval) (`Timeline|BumpAmount` :!via `PlayFromStart` :!label _label)
        (:`Update`
          (`SceneComponent.K2_SetRelativeLocation` (`self.Bumper Mechanism`) (`KismetMathLibrary.VLerp` (0.0 0.0 0.0) (0.0 0.0 -70.0) _bumpval) false false)
          (`LightComponent.SetIntensity` (`self.PointLight`) (`KismetMathLibrary.Lerp` 0.0 25000.0 _bumpval))
          (`MaterialInstanceDynamic.SetScalarParameterValue` (`self.BumperTopMat_Inst`) "EmissionBoost" (`KismetMathLibrary.Lerp` 0.0 100.0 _bumpval)) ; Making the sticker glow
        )))
    (:`CastFailed`
      (goto _label :!via `PlayFromStart`))))

(fn `UserConstructionScript`
  (bind _returnvalue (`PrimitiveComponent.CreateDynamicMaterialInstance` (`self.BumperHead`) 1 null "None"))
  (set `self.BumperTopMat_Inst` _returnvalue))